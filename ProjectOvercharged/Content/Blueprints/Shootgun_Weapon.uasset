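; Shotgun weapon Blueprint with limited ammo, a timed animated reload and a dry-fire sound when empty.
; Fire decrements ammo, plays randomized gunshot audio and animation unless reloading, then casts a single randomly spread ray from the player camera.
; The impact point places a bullet decal, while a tracer spawns from the weapon's scene point along camera rotation.
; A macro briefly flashes a point light and randomly rescaled muzzle plane.
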(event EventBeginPlay
  (|CallParentFunction) ; This node is disabled and will not be called.\nDrag off pins to build functionality.
)

(event Collision|EventActorBeginOverlap
  (params (OtherActor :type Actor%20Object%20Reference))
  (|CallParentFunction OtherActor) ; This node is disabled and will not be called.\nDrag off pins to build functionality.
)

(event EventTick
  (params (DeltaSeconds :type Float%20%28single-precision%29))
  (|CallParentFunction DeltaSeconds) ; This node is disabled and will not be called.\nDrag off pins to build functionality.
)

(event EventFire
  (if (> (Variables|Default|GetAmmoCount) 0)
    (CallFunction|AmmoCheck)
    (bind (_startlocation _impactpoint) (CallFunction|LineTrace))
    (CallFunction|SpawnDecalTracer _startlocation _impactpoint _impactpoint)
    (Utilities|NewMacro0)
    (else
      (Audio|PlaySoundatLocation "/Game/Sounds/Shooting/DryFire.DryFire" (Transformation|GetActorLocation) "0, 0, 0" 1.0 1.0 0.0 "/Game/Sounds/Shooting/ShootAttenuation.ShootAttenuation" "/Game/Sounds/Shooting/ShootConcurrency.ShootConcurrency" 0))))

(event EventReload
  (Components|Animation|PlayAnimation (Variables|Default|GetSkeletalMesh) 0 false)
  (Utilities|FlowControl|Delay (Variables|Default|GetReloadTime))
  (Variables|Default|SetAmmoCount (Variables|Default|GetMaxAmmo)))

(fn ConstructionScript
  (|CallParentFunction)
  (Variables|Default|SetMaxAmmo 7)
  (Variables|Default|SetAmmoCount 7)
  (Variables|Default|SetReloadTime 2.0)
  (Variables|Default|SetBulletSpray 5e+02))

(fn AmmoCheck
  (bind _returnvalue (Math|Random|RandomFloatinRange 0.7 1.2))
  (Math|Integer|DecrementInt (Variables|Default|GetAmmoCount)
    (:%20%20
      (if (not (Variables|/Game/FirstPersonBP/Blueprints/FirstPersonCharacter.FirstPersonCharacter_C|GetIsReload (.AsFirst%20Person%20Character (Utilities|Casting|CastToFirstPersonCharacter (Game|GetPlayerCharacter 0)))))
        (Audio|PlaySoundatLocation "/Game/Sounds/Shooting/Gunshot.Gunshot" (Transformation|GetActorLocation) "0, 0, 0" (* _returnvalue 2.5) _returnvalue 0.0 "/Game/Sounds/Shooting/ShootAttenuation.ShootAttenuation" "/Game/Sounds/Shooting/ShootConcurrency.ShootConcurrency" 0)
        (Components|Animation|PlayAnimation (Variables|Default|GetSkeletalMesh) 0 false)))))

(fn LineTrace
  (bind _returnvalue (Game|GetPlayerCharacter 0))
  (bind _bulletspray (Variables|Default|GetBulletSpray))
  (bind _scene (Variables|Default|GetScene))
  (bind _returnvalue_2 (Transformation|GetWorldLocation _scene))
  (bind _returnvalue_3 (* _bulletspray -1.0))
  (bind _asfirst_person_character (Utilities|Casting|CastToFirstPersonCharacter _returnvalue))
  (bind _firstpersoncamera (Variables|/Game/FirstPersonBP/Blueprints/FirstPersonCharacter.FirstPersonCharacter_C|GetFirstPersonCamera _asfirst_person_character))
  (bind _returnvalue_4 (Transformation|GetWorldLocation _firstpersoncamera))
  (bind _outhit (Collision|LineTraceByChannel _returnvalue_4 (+ (+ _returnvalue_4 (* (Math|Vector|GetForwardVector _firstpersoncamera) 2e+04)) (Math|Vector|MakeVector (Math|Random|RandomFloatinRange _returnvalue_3 _bulletspray) (Math|Random|RandomFloatinRange _returnvalue_3 _bulletspray) (Math|Random|RandomFloatinRange _returnvalue_3 _bulletspray))) "TraceTypeQuery1" false 0 "None"))
  (Collision|LineTraceByChannel _returnvalue_2 (.ImpactPoint (Collision|BreakHitResult _outhit)) "TraceTypeQuery1" false 0 "None" true "(R=0.000000,G=1.000000,B=0.172742,A=1.000000)")
  (return _returnvalue_2 (.ImpactPoint (Collision|BreakHitResult _outhit))))

(fn SpawnDecalTracer
  (params (Location :type Vector) (SpawnTransform :type Vector) (ImpactPoint :type Vector))
  (Game|SpawnActorfromClass "/Game/Blueprints/BulletDecal.BulletDecal_C" (Math|Transform|MakeTransform SpawnTransform (Math|Conversions|RotationFromXVector ImpactPoint) "0.100000,0.100000,0.100000") "Undefined" 0 0)
  (if (>= (Math|Random|RandomIntegerinRange 1 10) 0)
    (Game|SpawnActorfromClass "/Game/Blueprints/Tracer_BP.Tracer_BP_C" (Math|Transform|MakeTransform Location (Transformation|GetWorldRotation (Variables|/Game/FirstPersonBP/Blueprints/FirstPersonCharacter.FirstPersonCharacter_C|GetFirstPersonCamera (.AsFirst%20Person%20Character (Utilities|Casting|CastToFirstPersonCharacter (Game|GetPlayerCharacter 0))))) "0.100000,0.100000,0.100000") "Undefined" 0 0))
  (return))